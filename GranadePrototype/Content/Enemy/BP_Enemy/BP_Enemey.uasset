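; BP_Enemey is an enemy Blueprint with health, a damage reaction and a UI bar widget.
; On BeginPlay it creates an enemy bar widget, after a validity check, and adds it to the viewport.
; Its Damage function starts a looping pain animation, subtracts the amount from Health and destroys the actor at zero or below.
; The RadialDamage event is empty, and the debug prints are unconnected.
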(event `self.ReceiveBeginPlay`
  (`/Engine/EditorBlueprintResources/StandardMacros.IsValid` "BP_Enemey"
    (:`Is Valid`
      (bind _returnvalue (`|CreateWidget` "/Game/UI/BP_EnemyBar.BP_EnemyBar_C"))
      (`UserWidget.AddToViewport` _returnvalue 0))))

(event `self.ReceiveRadialDamage`
  (params (DamageReceived :type "Float (single-precision)") (DamageType :type "DamageType Object Reference") (Origin :type "Vector Structure") (HitInfo :type "HitResult Structure (by ref)") (InstigatedBy :type "Controller Object Reference") (DamageCauser :type "Actor Object Reference")))

(fn `Damage`
  (params (Amount :type "Float (double-precision)"))
  (`SkeletalMeshComponent.PlayAnimation` (`self.SkeletalMeshComponent`) "/Game/Enemy/Anim/Pain_Gesture.Pain_Gesture" true)
  (bind _output_get (set `self.Health` (- (`self.Health`) Amount)))
  (if (<= _output_get 0.0)
    (`self.K2_DestroyActor`)))

(fn `UserConstructionScript`)