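; BP_Friend is a friendly actor with a skeletal mesh and a health value that can be healed.
; On BeginPlay it adds a BP_FriendBar widget to the viewport if its BP_Friend reference is valid.
; Heal adds health while below maximum; on reaching it, health is set to a hardcoded 100 and the mesh loops Ninja_Idle.
; The radial damage event is empty, so this graph applies no damage.
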(event `self.ReceiveBeginPlay`
  (`/Engine/EditorBlueprintResources/StandardMacros.IsValid` "BP_Friend"
    (:`Is Valid`
      (bind _returnvalue (`|CreateWidget` "/Game/UI/BP_FriendBar.BP_FriendBar_C"))
      (`UserWidget.AddToViewport` _returnvalue 0))))

(event `self.ReceiveRadialDamage`
  (params (DamageReceived :type "Float (single-precision)") (DamageType :type "DamageType Object Reference") (Origin :type "Vector Structure") (HitInfo :type "HitResult Structure (by ref)") (InstigatedBy :type "Controller Object Reference") (DamageCauser :type "Actor Object Reference")))

(fn `Heal`
  (params (Amount :type "Float (double-precision)"))
  (if (< (`self.Health`) (`self.MaxHeatlhValue`))
    (bind _output_get (set `self.Health` (+ Amount (`self.Health`))))
    (if (>= _output_get (`self.MaxHeatlhValue`))
      (set `self.Health` 100.0)
      (`SkeletalMeshComponent.PlayAnimation` (`self.SkeletalMeshComponent`) "/Game/Friend/Anim/Ninja_Idle.Ninja_Idle" true))))

(fn `UserConstructionScript`)