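; Grenade projectile that detonates on a short timed fuse after it spawns.
; The construction script feeds the Strenght variable into the projectile movement's initial speed.
; BeginPlay waits, then Explode plays a sound and enlarged particle effect, spawns a scaled BP_Grenade_AOE actor at its location and destroys the grenade.
; Collision overlap does nothing, and some leftover debug and delayed-destroy nodes are unconnected.
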(event `self.Collision.OnComponentBeginOverlap`
  (params (OverlappedComponent :type "PrimitiveComponent Object Reference") (OtherActor :type "Actor Object Reference") (OtherComp :type "PrimitiveComponent Object Reference") (OtherBodyIndex :type Integer) (bFromSweep :type Boolean) (SweepResult :type "HitResult Structure (by ref)")))

(event `self.ReceiveBeginPlay`
  ;[1 1 1] Effects
  (`KismetSystemLibrary.Delay` 1.5)
  (`self.Explode`))

(event `self.ReceiveTick`
  (params (DeltaSeconds :type "Float (single-precision)")))

(fn `Explode`
  (bind _returnvalue (`self.K2_GetActorLocation`))
  (`GameplayStatics.SpawnSoundAtLocation` "/Game/Resources/StarterContent/Audio/Explosion01.Explosion01" _returnvalue (struct) 1.0 1.0 0.0 null null)
  (`GameplayStatics.SpawnEmitterAtLocation` "/Game/Resources/MilitaryWeapDark/FX/P_Grenade_MuzzleFlash_01.P_Grenade_MuzzleFlash_01" _returnvalue (struct) (5.0 5.0 5.0))
  (`|SpawnActorFromClass` "/Game/BP_Grenade/BP_Grenade_AOE.BP_Grenade_AOE_C" (`KismetMathLibrary.MakeTransform` _returnvalue (struct) (5.0 5.0 5.0)) "Undefined" "OverrideRootScale" null null)
  (`self.K2_DestroyActor`))

(fn `UserConstructionScript`
  (set `ProjectileMovementComponent.InitialSpeed` (`self.Strenght`) (`self.ProjectileMovement`)))