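; Grenade area-of-effect actor that damages enemies and heals friends inside its collider, destroying itself four seconds after spawning.
; On overlap, actor tags select a cast to BP_Enemey or BP_Friend and start a looping damage or heal timer.
; End-overlap events bound on the target aim to stop that timer, which also clears if the target becomes invalid.
; Only one enemy and one friend reference are stored, each overwritten by newer overlaps.
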(event `OnEnemyEndOverlap` :!signature `self.OnActorEndOverlap`
  (params (OverlappedActor :type "Actor Object Reference") (OtherActor :type "Actor Object Reference"))
  ;[1 1 1] Enemy
  ;;[0.1311 0.7865 0.6806] To Avoid Damage Out of the AOE
  (if (== OverlappedActor self)
    (`KismetSystemLibrary.K2_ClearAndInvalidateTimerHandle` (stale `self.Collider.OnComponentBeginOverlap` _returnvalue))))

(event `self.ReceiveBeginPlay`
  (`KismetSystemLibrary.Delay` 4.0)
  (`self.K2_DestroyActor`))

(event `OnDamageTick`
  ;[1 1 1] Enemy
  (`/Engine/EditorBlueprintResources/StandardMacros.IsValid` (stale `self.Collider.OnComponentBeginOverlap` _asbp_enemey)
    (:`Is Valid`
      (`/Game/Enemy/BP_Enemy/BP_Enemey.Damage` (stale `self.Collider.OnComponentBeginOverlap` _asbp_enemey) (`self.DamageAmount`)))
    (:`Is Not Valid`
      (`KismetSystemLibrary.K2_ClearAndInvalidateTimerHandle` (stale `self.Collider.OnComponentBeginOverlap` _returnvalue)))))

(event `self.Collider.OnComponentBeginOverlap`
  (params (OverlappedComponent :type "PrimitiveComponent Object Reference") (OtherActor :type "Actor Object Reference") (OtherComp :type "PrimitiveComponent Object Reference") (OtherBodyIndex :type Integer) (bFromSweep :type Boolean) (SweepResult :type "HitResult Structure (by ref)"))
  (for _array_element (`Actor.Tags` OtherActor)
    (switch `name` _array_element
      (:`Enemy`
        ;[1 1 1] Enemy
        (bind _asbp_enemey (cast `/Game/Enemy/BP_Enemy/BP_Enemey` OtherActor))
        (bind _returnvalue (`KismetSystemLibrary.K2_SetTimerDelegate` (delegate `OnDamageTick`) 0.5 true))
        (add `self.OnActorEndOverlap` _asbp_enemey (delegate `OnEnemyEndOverlap`)))
      (:`Friend`
        ;[1 1 1] Friend
        (bind _asbp_friend (cast `/Game/Friend/BP_Friend/BP_Friend` OtherActor))
        (bind _returnvalue_2 (`KismetSystemLibrary.K2_SetTimerDelegate` (delegate `OnHealTick`) 0.5 true))
        (add `self.OnActorEndOverlap` _asbp_friend (delegate `OnFriendEndOverlap`))))))

(event `self.Collider.OnComponentEndOverlap`
  (params (OverlappedComponent :type "PrimitiveComponent Object Reference") (OtherActor :type "Actor Object Reference") (OtherComp :type "PrimitiveComponent Object Reference") (OtherBodyIndex :type Integer)))

(event `OnFriendEndOverlap` :!signature `self.OnActorEndOverlap`
  (params (OverlappedActor :type "Actor Object Reference") (OtherActor :type "Actor Object Reference"))
  ;[1 1 1] Friend
  ;;[0.1311 0.7865 0.6806] To Avoid Damage Out of the AOE
  (if (== OverlappedActor self)
    (`KismetSystemLibrary.K2_ClearAndInvalidateTimerHandle` (stale `self.Collider.OnComponentBeginOverlap` _returnvalue_2))))

(event `OnHealTick`
  ;[1 1 1] Friend
  (`/Engine/EditorBlueprintResources/StandardMacros.IsValid` (stale `self.Collider.OnComponentBeginOverlap` _asbp_friend)
    (:`Is Valid`
      (`/Game/Friend/BP_Friend/BP_Friend.Heal` (stale `self.Collider.OnComponentBeginOverlap` _asbp_friend) (`self.HealthAmount`)))
    (:`Is Not Valid`
      (`KismetSystemLibrary.K2_ClearAndInvalidateTimerHandle` (stale `self.Collider.OnComponentBeginOverlap` _returnvalue_2)))))

(fn `UserConstructionScript`)